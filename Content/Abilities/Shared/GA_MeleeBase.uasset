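; GA_MeleeBase is a shared Gameplay Ability for melee attacks that plays a montage and applies a damage effect.
; On activation it commits, plays the montage and waits once for the Skill.Melee.DealDamage gameplay event.
; That event's target receives the configured GameplayEffect at the ability's level, which a comment says comes from the weapon item.
; The ability ends when the montage completes, blends out, is interrupted or is cancelled.
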(event `self.K2_ActivateAbility`
  (`|ExecutionSequence`
    (:`then_0`
      (`self.K2_CommitAbility`))
    (:`then_1`
      (`AbilityTask_PlayMontageAndWait.CreatePlayMontageAndWaitProxy` "None" (`self.MontageToPlay`)
        (:`OnCompleted`
          _)
        (:`OnBlendOut`
          _)
        (:`OnInterrupted`
          _)
        (:`OnCancelled`
          _))
      (`self.K2_EndAbility`))
    (:`then_2`
      (bind (_asynctaskproxy _payload) (`AbilityTask_WaitGameplayEvent.WaitGameplayEvent` (struct :`TagName` "Skill.Melee.DealDamage") null true)
        (:`EventReceived`
          (`self.BP_ApplyGameplayEffectToTarget` (`AbilitySystemBlueprintLibrary.AbilityTargetDataFromActor` (`.Target` (break `GameplayEventData` _payload))) (`self.GameplayEffect`) (`self.GetAbilityLevel`)))))))