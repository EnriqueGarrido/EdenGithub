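; Base Gameplay Ability, shared by name and path, that plays a montage and then fires a projectile from the avatar.
; It commits without checking the result, spawns the projectile ahead of the avatar on montage completion or blend out, and ends without spawning on interruption or cancel.
; The projectile receives the avatar pawn as instigator and a gameplay effect spec built at the ability's level.
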(event `self.K2_ActivateAbility`
  (bind _returnvalue (`self.GetAvatarActorFromActorInfo`))
  (`|ExecutionSequence`
    (:`then_0`
      (`self.K2_CommitAbility`))
    (:`then_1`
      (`AbilityTask_PlayMontageAndWait.CreatePlayMontageAndWaitProxy` "None" (`self.MontageToPlay`)
        (:`OnCompleted`
          (`|SpawnActorFromClass` (`self.ProjectileClass`) (`KismetMathLibrary.MakeTransform` (+ (`Actor.K2_GetActorLocation` _returnvalue) (* (`Actor.GetActorForwardVector` _returnvalue) 260.0)) (`Actor.K2_GetActorRotation` _returnvalue)) "Undefined" "OverrideRootScale" null (`self.MakeOutgoingGameplayEffectSpec` (`self.GameplayEffect`) (`KismetMathLibrary.Conv_IntToDouble` (`self.GetAbilityLevel`))) (cast `Pawn` _returnvalue :!pure true) :!label _label)
          (`self.K2_EndAbility`))
        (:`OnBlendOut`
          (goto _label))
        (:`OnInterrupted`
          (`self.K2_EndAbility` :!label _label_2))
        (:`OnCancelled`
          (goto _label_2))))))