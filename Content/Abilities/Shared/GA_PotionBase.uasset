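; GA_PotionBase is a base gameplay ability for using a potion.
; On activation it commits, plays a montage and waits once for the Skill.Potion.UseItem gameplay event.
; That event applies the configured gameplay effect to the owner at the ability level, then consumes the potion through a hardcoded slot on BP_PlayerController.
; The ability ends when the montage completes, blends out, or is interrupted or cancelled.
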(event `self.K2_ActivateAbility`
  (bind (_returnvalue_owneractor _returnvalue_avataractor _returnvalue_playercontroller) (break `GameplayAbilityActorInfo` (`self.GetActorInfo`)))
  (`|ExecutionSequence`
    (:`then_0`
      (`self.K2_CommitAbility`))
    (:`then_1`
      (`AbilityTask_PlayMontageAndWait.CreatePlayMontageAndWaitProxy` "None" (`self.MontageToPlay`)
        (:`OnCompleted`
          _)
        (:`OnBlendOut`
          _)
        (:`OnInterrupted`
          _)
        (:`OnCancelled`
          _))
      (`self.K2_EndAbility`))
    (:`then_2`
      (`AbilityTask_WaitGameplayEvent.WaitGameplayEvent` (struct :`TagName` "Skill.Potion.UseItem") null true
        (:`EventReceived`
          (`self.BP_ApplyGameplayEffectToOwner` (`self.GameplayEffect`) (`self.GetAbilityLevel`))
          ;[1 1 1] Consume potion item from inventory
          (bind _asbp_player_controller (cast `/Game/Blueprints/BP_PlayerController` _returnvalue_playercontroller))
          (`EdenValleyPlayerController.SetSlottedItem` _asbp_player_controller 4 null))))))