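; Player Ground Blast ability: a confirm-to-cast, ground-targeted attack that damages targets and launches enemies upward.
; Activation flags the player as targeting, plays an aim montage and waits for confirmation through the BP_GroundBlastActor target actor.
; On confirm it commits, plays the cast montage, spawns storm effects at the target point, applies level-scaled damage and pushes BP_EnemyBase targets upward.
; The ability ends after the blast or on cancel.
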(event `self.K2_ActivateAbility`
  (`|ExecutionSequence`
    (:`then_0`
      (set `/Game/Blueprints/BP_PlayerCharacter.bIsTargeting` true (`/Game/Blueprints/BP_FunctionLibrary.GetPlayerCharacterBP`)))
    (:`then_1`
      (`AbilityTask_PlayMontageAndWait.CreatePlayMontageAndWaitProxy` "None" "/Game/Characters/Animations/MagicWandStance/AM_GroundBlast.AM_GroundBlast"
        (:`then`
          (`KismetSystemLibrary.Delay` (`AnimSequenceBase.SequenceLength` (`self.GetCurrentMontage`))))))
    (:`then_2`
      (bind (_asynctaskproxy _data) (`AbilityTask_WaitTargetData.WaitTargetData` "None" "UserConfirmed" "/Game/Abilities/Player/Skills/GroundBlast/BP_GroundBlastActor.BP_GroundBlastActor_C" (struct) (struct) null)
        (:`ValidData`
          (`self.K2_CommitAbility`)
          (`AbilityTask_PlayMontageAndWait.CreatePlayMontageAndWaitProxy` "None" "/Game/Characters/Animations/MagicWandStance/AM_GroundBlastCast.AM_GroundBlastCast"
            (:`then`
              (bind _returnvalue (`AbilitySystemBlueprintLibrary.GetTargetDataEndPoint` _data (- (`AbilitySystemBlueprintLibrary.GetDataCountFromTargetData` _data) 1)))
              (`GameplayStatics.SpawnEmitterAtLocation` "/Game/Effects/Particles/P_ky_storm.P_ky_storm" _returnvalue)
              (`GameplayStatics.SpawnSoundAtLocation` "/Game/Sounds/Effects/EffectsElements/Wavs/tornado-4s.tornado-4s" _returnvalue (struct) 0.6 1.0 0.0 null null)
              (`self.BP_ApplyGameplayEffectToTarget` _data "/Game/Abilities/Player/Skills/GroundBlast/GE_GroundBlastDamage.GE_GroundBlastDamage_C" (`self.GetAbilityLevel`))
              (for _array_element (`AbilitySystemBlueprintLibrary.GetActorsFromTargetData` _data)
                (if (`KismetMathLibrary.ClassIsChildOf` (`GameplayStatics.GetObjectClass` _array_element) "/Game/Blueprints/NPC/Enemies/BP_EnemyBase.BP_EnemyBase_C")
                  (bind _asbp_enemy_base (cast `/Game/Blueprints/NPC/Enemies/BP_EnemyBase` _array_element))
                  (`/Game/Blueprints/NPC/Enemies/BP_EnemyBase.PushCharacter` _asbp_enemy_base (0.0 0.0 150.0) 4.0)))
              (`self.K2_EndAbility`))))
        (:`Cancelled`
          (`self.K2_EndAbility`))))))