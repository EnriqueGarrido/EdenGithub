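; Player dash Gameplay Ability that launches the character forward and damages a target along the way.
; On activation it commits, zeroes ground friction, applies a forward velocity impulse and sets pawn collision to overlap.
; During the dash montage, a one-shot DealDamage gameplay event applies the dash damage effect to its target at ability level.
; Montage completion, blend-out, interruption or cancellation restores friction and blocking collision, then ends the ability.
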(event `self.K2_ActivateAbility`
  (`|ExecutionSequence`
    (:`then_0`
      (`self.K2_CommitAbility`))
    (:`then_1`
      (bind _ascharacter (cast `Character` (`self.GetOwningActorFromActorInfo`))
        (:`then`
          (bind _charactermovement (`Character.CharacterMovement` _ascharacter))
          (set `self.OriginalGroundFriction` (`CharacterMovementComponent.GroundFriction` _charactermovement))
          (set `CharacterMovementComponent.GroundFriction` 0.0 _charactermovement)
          (`CharacterMovementComponent.AddImpulse` _charactermovement (* (`Actor.GetActorForwardVector` _ascharacter) 2000.0) true))
        (:`CastFailed`
          (`self.K2_EndAbility`))))
    (:`then_2`
      (`/Game/Blueprints/BP_PlayerCharacter.SetCollisonToPawn` (`/Game/Blueprints/BP_FunctionLibrary.GetPlayerCharacterBP`) "ECR_Overlap"))
    (:`then_3`
      (`AbilityTask_PlayMontageAndWait.CreatePlayMontageAndWaitProxy` "None" "/Game/Characters/Animations/NoWeaponStance/AM_DashForward_noWeaponAnim.AM_DashForward_noWeaponAnim"
        (:`then`
          (bind (_asynctaskproxy _payload) (`AbilityTask_WaitGameplayEvent.WaitGameplayEvent` (struct :`TagName` "Skill.Dash.DealDamage") null true)
            (:`EventReceived`
              (`self.BP_ApplyGameplayEffectToTarget` (`AbilitySystemBlueprintLibrary.AbilityTargetDataFromActor` (`.Target` (break `GameplayEventData` _payload))) "/Game/Abilities/Player/Skills/Dash/GE_DashDamage.GE_DashDamage_C" (`self.GetAbilityLevel`)))))
        (:`OnCompleted`
          (set `CharacterMovementComponent.GroundFriction` (`self.OriginalGroundFriction`) _charactermovement :!label _label)
          (`/Game/Blueprints/BP_PlayerCharacter.SetCollisonToPawn` (`/Game/Blueprints/BP_FunctionLibrary.GetPlayerCharacterBP`) "ECR_Block")
          (`self.K2_EndAbility`))
        (:`OnBlendOut`
          (goto _label))
        (:`OnInterrupted`
          (goto _label))
        (:`OnCancelled`
          (goto _label))))))