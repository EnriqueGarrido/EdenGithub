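; Sound manager Blueprint that plays background music, a looping-free random playlist, plus an SFX source and final battle music.
; On BeginPlay it starts the SFX source and fades in a random song immediately.
; AudioSource's OnAudioFinished picks another song, waiting a random delay before fading it in.
; Separate events fade the battle song in and out on the same AudioSource; Tick-based timing logic is disconnected.
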(event `self.ReceiveBeginPlay`
  ;[0 0 0] Init first song
  (`self.RandomMusicStart` true)
  ;[0 0 0] Background effect playing
  (`AudioComponent.Play` (`self.SFXSource`) 0.0))

(event `self.AudioSource.OnAudioFinished`
  ;[0 0 0] Controls when an audio is Finished
  (`self.RandomMusicStart` false))

(event `self.ReceiveTick`
  (params (DeltaSeconds :type "Float (single-precision)")))

(event `RandomMusicStart`
  (params (`Instant?` :type Boolean))
  (bind _randomsongs (`self.RandomSongs`))
  (bind _audiosource (`self.AudioSource`))
  ;[0 0 0] Plays the sound after a centain delay is instantly
  (`AudioComponent.SetSound` _audiosource (`|GetArrayItem` _randomsongs (`KismetMathLibrary.RandomInteger` (`KismetArrayLibrary.Array_Length` _randomsongs))))
  (if (not `Instant?`)
    (bind _output_get (set `self.NextSongTime` (`KismetMathLibrary.RandomFloatInRange` (`self.MinTimeBetweenSongs`) (`self.MaxTimeBetweenSongs`))))
    (`KismetSystemLibrary.Delay` _output_get))
  (`AudioComponent.FadeIn` _audiosource 5.0 1.0 0.0))

(event `PlayFinalBattleMusic`
  (bind _audiosource (`self.AudioSource`))
  ;[0 0 0] Calles for final mission musics
  (`AudioComponent.SetSound` _audiosource (`self.BattleSong`))
  (`AudioComponent.FadeIn` _audiosource 5.0 1.0 0.0))

(event `EndFinalBattleMusic`
  ;[0 0 0] Calles for final mission musics
  (`AudioComponent.FadeOut` (`self.AudioSource`) 2.5 0.0))

(fn `UserConstructionScript`)