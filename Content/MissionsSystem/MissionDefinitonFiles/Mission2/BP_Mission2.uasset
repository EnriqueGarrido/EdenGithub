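; Mission Blueprint for the second mission, which sets up an enemy encounter and equips the player for it.
; When the mission is added, it has the game mode set target points and spawn enemies, then grants a weapon and a shield.
; Both items are looked up by row name in the game state's weapon data table and added to inventory through the player controller.
; Finishing the mission sets the game instance's active mission to the pottery mission.
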(event `self.ReceiveBeginPlay`
  (`parent.ReceiveBeginPlay`))

(event `/Game/MissionsSystem/MissionGeneralFiles/ProjectFiles/Interfaces/BPI_InteractionInterface.On Missions Added`
  (bind _gamemode (`/Game/Blueprints/BP_FunctionLibrary.GetGameModeBP`))
  (`/Game/Blueprints/BP_GameModeBase.SetTargetPoints` _gamemode)
  (`/Game/Blueprints/BP_GameModeBase.SpawnEnemy` _gamemode 4)
  (`self.AddWeapon`)
  (`self.AddShield`))

(event `self.OnFinishMision`
  (set `/Game/Blueprints/BP_GameInstance.missionActive` "PotteryMission" (`/Game/Blueprints/BP_FunctionLibrary.GetGameInstanceBP`)))

(fn `AddShield`
  (bind _returnvalue (`|GetDataTableRow` (`EdenValleyGameStateBase.GetWeaponDB` (`/Game/Blueprints/BP_FunctionLibrary.GetGameStateBP`)) (`self.Shield`))
    (:`then`
      (bind (_weaponactor _itemtype _itemid) (break `EdenValleyWeaponItem` _returnvalue))
      (`EdenValleyPlayerController.AddItemToInventoryByID` (`/Game/Blueprints/BP_FunctionLibrary.GetPlayerControllerBP`) _itemtype _itemid 1))))

(fn `AddWeapon`
  (bind _returnvalue (`|GetDataTableRow` (`EdenValleyGameStateBase.GetWeaponDB` (`/Game/Blueprints/BP_FunctionLibrary.GetGameStateBP`)) (`self.Weapon`))
    (:`then`
      (bind (_weaponactor _itemtype _itemid) (break `EdenValleyWeaponItem` _returnvalue))
      (`EdenValleyPlayerController.AddItemToInventoryByID` (`/Game/Blueprints/BP_FunctionLibrary.GetPlayerControllerBP`) _itemtype _itemid 1))))

(fn `UserConstructionScript`
  (`parent.UserConstructionScript`))