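; Mission 4 Blueprint that runs setup when the mission is added and advances the story when it finishes.
; On add, it looks up its Ability row in the game state's skill DataTable, grants that item to the player controller's inventory, and calls the game mode's SpawnEnemy.
; On finish, it sets the game instance's active mission to "The Eden end?".
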(event `/Game/MissionsSystem/MissionGeneralFiles/ProjectFiles/Interfaces/BPI_InteractionInterface.On Missions Added`
  (`self.AddAbility`)
  (`/Game/Blueprints/BP_GameModeBase.SpawnEnemy` (`/Game/Blueprints/BP_FunctionLibrary.GetGameModeBP`) 14))

(event `self.OnFinishMision`
  (set `/Game/Blueprints/BP_GameInstance.missionActive` "The Eden end?" (`/Game/Blueprints/BP_FunctionLibrary.GetGameInstanceBP`)))

(fn `AddAbility`
  (bind _returnvalue (`|GetDataTableRow` (`EdenValleyGameStateBase.GetSkillDB` (`/Game/Blueprints/BP_FunctionLibrary.GetGameStateBP`)) (`self.Ability`))
    (:`then`
      (bind (_itemtype _itemid) (break `EdenValleySkillItem` _returnvalue))
      (`EdenValleyPlayerController.AddItemToInventoryByID` (`/Game/Blueprints/BP_FunctionLibrary.GetPlayerControllerBP`) _itemtype _itemid 1))))

(fn `UserConstructionScript`
  (`parent.UserConstructionScript`))