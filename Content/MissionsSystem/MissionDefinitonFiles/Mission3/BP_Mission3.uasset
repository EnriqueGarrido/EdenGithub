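; BP_Mission3 defines the third mission, a mushroom-collecting quest in the mission system.
; When added, it sets target points if needed and has the game mode spawn mushrooms.
; On finish it grants health and mana potions looked up in the potion data table, then deducts fixed counts of five mushroom types from the inventory.
; Finally it sets the game instance's active mission to "The power of skills".
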(event `/Game/MissionsSystem/MissionGeneralFiles/ProjectFiles/Interfaces/BPI_InteractionInterface.On Missions Added`
  (`self.SetTargetPointsIfNeeded`)
  (`/Game/Blueprints/BP_GameModeBase.SpawnMushrooms` (`/Game/Blueprints/BP_FunctionLibrary.GetGameModeBP`)))

(event `self.OnFinishMision`
  (`self.AddHealthPotion`)
  (`self.AddManaPotion`)
  (`self.RemoveMushrooms`)
  (set `/Game/Blueprints/BP_GameInstance.missionActive` "The power of skills" (`/Game/Blueprints/BP_FunctionLibrary.GetGameInstanceBP`)))

(fn `AddHealthPotion`
  (bind _returnvalue (`|GetDataTableRow` (`EdenValleyGameStateBase.GetPotionDB` (`/Game/Blueprints/BP_FunctionLibrary.GetGameStateBP`)) (`self.HealthPotion`))
    (:`then`
      (bind (_itemtype _itemid) (break `EdenValleyPotionItem` _returnvalue))
      (`EdenValleyPlayerController.AddItemToInventoryByID` (`/Game/Blueprints/BP_FunctionLibrary.GetPlayerControllerBP`) _itemtype _itemid 2))))

(fn `AddManaPotion`
  (bind _returnvalue (`|GetDataTableRow` (`EdenValleyGameStateBase.GetPotionDB` (`/Game/Blueprints/BP_FunctionLibrary.GetGameStateBP`)) (`self.ManaPotion`))
    (:`then`
      (bind (_itemtype _itemid) (break `EdenValleyPotionItem` _returnvalue))
      (`EdenValleyPlayerController.AddItemToInventoryByID` (`/Game/Blueprints/BP_FunctionLibrary.GetPlayerControllerBP`) _itemtype _itemid 2))))

(fn `RemoveMushrooms`
  (bind _playercontroller (`/Game/Blueprints/BP_FunctionLibrary.GetPlayerControllerBP`))
  (for _array_element (`EdenValleyPlayerController.GetOtherInventory` (`/Game/Blueprints/BP_FunctionLibrary.GetPlayerControllerBP`))
    (switch `name` (`.ItemID` (break `EdenValleyItem` (`EdenValleyItemData.Item` _array_element)))
      (:`YellowMushroom`
        (`EdenValleyPlayerController.SetInventoryItemCount` _playercontroller _array_element -2))
      (:`LittleMushroom`
        (`EdenValleyPlayerController.SetInventoryItemCount` _playercontroller _array_element -4))
      (:`BrownMushroom`
        (`EdenValleyPlayerController.SetInventoryItemCount` _playercontroller _array_element -3))
      (:`WhiteMushroom`
        (`EdenValleyPlayerController.SetInventoryItemCount` _playercontroller _array_element -5))
      (:`RedMushroom`
        (`EdenValleyPlayerController.SetInventoryItemCount` _playercontroller _array_element -4)))))

(fn `UserConstructionScript`
  (`parent.UserConstructionScript`))