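; Master monster for the mission system that optionally wanders to random navigable points, takes damage, and reports itself to the objective manager.
; On death it notifies the mission manager, deregisters and disables capsule collision.
; EnemyChecker overlaps pass or clear the enemy reference for interface-implementing actors.
; Exiting the RespawnDistance-sized DistanceChecker box restores health, or delays then respawns or destroys a dead monster.
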(event `self.ReceiveBeginPlay`
  (set `self.CurrentHealth` (`self.MaxHealth`))
  (`KismetSystemLibrary.Delay` 0.2)
  (`/Game/MissionsSystem/MissionGeneralFiles/ProjectFiles/Interfaces/BPI_ObjectivesInterface.Assign Monsters` (`/Game/MissionsSystem/MissionGeneralFiles/ProjectFiles/Interfaces/BPI_Manager.Get Objective Manager`) (`self.MonsterInfo`))
  (if (and (`self.MoveToRandomLocations`) (not (`self.Dead?`))) :!label _label
    (`|AIMoveTo` self (`NavigationSystemV1.K2_GetRandomLocationInNavigableRadius` (`self.K2_GetActorLocation` self) (`self.RandomLocationRange`) null null) null
      (:`OnSuccess`
        (`KismetSystemLibrary.Delay` (`self.MoveDelay`))
        (goto _label)))))

(event `self.ReceiveAnyDamage`
  (params (Damage :type "Float (single-precision)") (DamageType :type "DamageType Object Reference") (InstigatedBy :type "Controller Object Reference") (DamageCauser :type "Actor Object Reference"))
  (if (not (`self.Dead?`))
    (bind _output_get (set `self.CurrentHealth` (- (`self.CurrentHealth`) Damage)))
    (if (<= _output_get 0.0)
      (set `self.Dead?` true)
      (message `/Game/MissionsSystem/MissionGeneralFiles/ProjectFiles/Interfaces/BPI_ObjectivesInterface.Set Enemy As Dead` (`self.Get Anim Instance`) "None" true)
      (`/Game/MissionsSystem/MissionGeneralFiles/ProjectFiles/Interfaces/BPI_EventInterface.Killed Monster Info` (`/Game/MissionsSystem/MissionGeneralFiles/ProjectFiles/Interfaces/BPI_Manager.Get Mission Manager`) (`GameplayStatics.GetObjectClass` self))
      (`/Game/MissionsSystem/MissionGeneralFiles/ProjectFiles/Interfaces/BPI_ObjectivesInterface.Remove Monsters` (`/Game/MissionsSystem/MissionGeneralFiles/ProjectFiles/Interfaces/BPI_Manager.Get Objective Manager`) (`self.MonsterInfo`))
      (`PrimitiveComponent.SetCollisionEnabled` (`self.CapsuleComponent`) "NoCollision"))))

(event `self.ReceiveEndPlay`
  (params (EndPlayReason :type "EEndPlayReason Enum" :default "Destroyed"))
  (bind _objective (`/Game/MissionsSystem/MissionGeneralFiles/ProjectFiles/Interfaces/BPI_Manager.Get Objective Manager`))
  (switch `EEndPlayReason` EndPlayReason
    (:`Destroyed`
      _)
    (:`RemovedFromWorld`
      _))
  (`/Engine/EditorBlueprintResources/StandardMacros.IsValid` (`KismetSystemLibrary.Conv_InterfaceToObject` _objective)
    (:`Is Valid`
      (`/Game/MissionsSystem/MissionGeneralFiles/ProjectFiles/Interfaces/BPI_ObjectivesInterface.Remove Monsters` _objective (`self.MonsterInfo`)))))

(event `self.EnemyChecker.OnComponentBeginOverlap`
  (params (OverlappedComponent :type "PrimitiveComponent Object Reference") (OtherActor :type "Actor Object Reference") (OtherComp :type "PrimitiveComponent Object Reference") (OtherBodyIndex :type Integer) (bFromSweep :type Boolean) (SweepResult :type "HitResult Structure (by ref)"))
  (if (and (`KismetSystemLibrary.DoesImplementInterface` OtherActor "/Game/MissionsSystem/MissionGeneralFiles/ProjectFiles/Interfaces/BPI_EventInterface.BPI_EventInterface_C") (not (`self.Dead?`)))
    (`/Game/MissionsSystem/MissionGeneralFiles/ProjectFiles/Interfaces/BPI_ObjectivesInterface.Pass Enemy Reference` (`/Game/MissionsSystem/MissionGeneralFiles/ProjectFiles/Interfaces/BPI_Manager.Get Objective Manager`) self)))

(event `self.EnemyChecker.OnComponentEndOverlap`
  (params (OverlappedComponent :type "PrimitiveComponent Object Reference") (OtherActor :type "Actor Object Reference") (OtherComp :type "PrimitiveComponent Object Reference") (OtherBodyIndex :type Integer))
  (if (`KismetSystemLibrary.DoesImplementInterface` OverlappedComponent "/Game/MissionsSystem/MissionGeneralFiles/ProjectFiles/Interfaces/BPI_EventInterface.BPI_EventInterface_C")
    (`/Game/MissionsSystem/MissionGeneralFiles/ProjectFiles/Interfaces/BPI_ObjectivesInterface.Remove Enemy Reference` (`/Game/MissionsSystem/MissionGeneralFiles/ProjectFiles/Interfaces/BPI_Manager.Get Objective Manager`))))

(event `self.DistanceChecker.OnComponentBeginOverlap`
  (params (OverlappedComponent :type "PrimitiveComponent Object Reference") (OtherActor :type "Actor Object Reference") (OtherComp :type "PrimitiveComponent Object Reference") (OtherBodyIndex :type Integer) (bFromSweep :type Boolean) (SweepResult :type "HitResult Structure (by ref)"))
  (if (`KismetSystemLibrary.DoesImplementInterface` OtherActor "/Game/MissionsSystem/MissionGeneralFiles/ProjectFiles/Interfaces/BPI_EventInterface.BPI_EventInterface_C")
    (set `self.OutsideOfTheBox` false)))

(event `self.DistanceChecker.OnComponentEndOverlap`
  (params (OverlappedComponent :type "PrimitiveComponent Object Reference") (OtherActor :type "Actor Object Reference") (OtherComp :type "PrimitiveComponent Object Reference") (OtherBodyIndex :type Integer))
  (if (`KismetSystemLibrary.DoesImplementInterface` OtherActor "/Game/MissionsSystem/MissionGeneralFiles/ProjectFiles/Interfaces/BPI_EventInterface.BPI_EventInterface_C")
    (set `self.OutsideOfTheBox` true)
    (if (`self.Dead?`)
      (`KismetSystemLibrary.Delay` (`self.RespawnTime`) :!label _label_2)
      (if (`self.OutsideOfTheBox`)
        (if (`self.RespawnEnemyAfterDeath?`)
          (set `self.CurrentHealth` (`self.MaxHealth`))
          (set `self.Dead?` false)
          (message `/Game/MissionsSystem/MissionGeneralFiles/ProjectFiles/Interfaces/BPI_ObjectivesInterface.Set Enemy As Dead` (`self.Get Anim Instance`) "None" false)
          (`/Game/MissionsSystem/MissionGeneralFiles/ProjectFiles/Interfaces/BPI_ObjectivesInterface.Assign Monsters` (`/Game/MissionsSystem/MissionGeneralFiles/ProjectFiles/Interfaces/BPI_Manager.Get Objective Manager`) (`self.MonsterInfo`))
          (`PrimitiveComponent.SetCollisionEnabled` (`self.CapsuleComponent`) "QueryAndPhysics")
          (else
            (`/Game/MissionsSystem/MissionGeneralFiles/ProjectFiles/Interfaces/BPI_ObjectivesInterface.Remove Monsters` (`/Game/MissionsSystem/MissionGeneralFiles/ProjectFiles/Interfaces/BPI_Manager.Get Objective Manager`) (`self.MonsterInfo`))
            (`self.K2_DestroyActor`)))
        (else
          (goto _label_2)))
      (else
        (set `self.CurrentHealth` (`self.MaxHealth`))))))

(fn `UserConstructionScript`
  (bind (_monsterinfo_monsterclass _monsterinfo_monstername _monsterinfo_amount _monsterinfo_addmarker_ _monsterinfo_displaymarkeronscreen_ _monsterinfo_meterstoaddmarker _monsterinfo_customizemarker) (break `/Game/MissionsSystem/MissionGeneralFiles/ProjectFiles/Structures/ActorStructures/BPS_MonsterInfo` (`self.MonsterInfo`)))
  (bind _respawndistance (`self.RespawnDistance`))
  (`BoxComponent.SetBoxExtent` (`self.DistanceChecker`) (`KismetMathLibrary.MakeVector` _respawndistance _respawndistance _respawndistance) true)
  (set `self.MonsterInfo` (make `/Game/MissionsSystem/MissionGeneralFiles/ProjectFiles/Structures/ActorStructures/BPS_MonsterInfo` (`GameplayStatics.GetObjectClass` self) _monsterinfo_monstername _monsterinfo_amount _monsterinfo_addmarker_ _monsterinfo_displaymarkeronscreen_ _monsterinfo_meterstoaddmarker _monsterinfo_customizemarker self)))