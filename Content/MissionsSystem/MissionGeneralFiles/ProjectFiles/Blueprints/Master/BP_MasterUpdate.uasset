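; Master mission-update trigger that shows a notification through the mission manager when a qualifying actor enters its box.
; Overlaps count only for actors implementing BPI_EventInterface, with a DoOnce flag that routes execution through a DoOnce gate.
; The notification takes its text, display time and border color from the Blueprint's variables.
; The construction script sizes the box from OverlapBoxExtent, forcing a fixed vertical extent.
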(event `self.Box.OnComponentBeginOverlap`
  (params (OverlappedComponent :type "PrimitiveComponent Object Reference") (OtherActor :type "Actor Object Reference") (OtherComp :type "PrimitiveComponent Object Reference") (OtherBodyIndex :type Integer) (bFromSweep :type Boolean) (SweepResult :type "HitResult Structure (by ref)"))
  (if (`KismetSystemLibrary.DoesImplementInterface` OtherActor "/Game/MissionsSystem/MissionGeneralFiles/ProjectFiles/Interfaces/BPI_EventInterface.BPI_EventInterface_C")
    (if (`self.DoOnce?`)
      (`/Engine/EditorBlueprintResources/StandardMacros.DoOnce` false
        (:`Completed`
          _)))
    (`/Game/MissionsSystem/MissionGeneralFiles/ProjectFiles/Interfaces/BPI_EventInterface.Update Notification` (`/Game/MissionsSystem/MissionGeneralFiles/ProjectFiles/Interfaces/BPI_Manager.Get Mission Manager`) (`self.DisplayTime`) (`self.Description`) (`self.BorderColor`))))

(fn `UserConstructionScript`
  (bind (_overlapboxextent_x _overlapboxextent_y) (`KismetMathLibrary.BreakVector` (`self.OverlapBoxExtent`)))
  (bind _output_get (set `self.OverlapBoxExtent` (`KismetMathLibrary.MakeVector` _overlapboxextent_x _overlapboxextent_y 150.0)))
  (`BoxComponent.SetBoxExtent` (`self.Box`) _output_get true))