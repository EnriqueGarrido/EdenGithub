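; Master mission actor that offers missions to the player or acts as an interaction target for them.
; Construction loads missions from a data table and configures it as either a visible blocking NPC or an invisible overlap trigger with particles.
; Box overlaps pass its reference to the mission manager and highlight it, while interaction opens the mission panel or reports the target.
; It registers with the objective manager on play, which it leaves when destroyed.
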(event `/Game/MissionsSystem/MissionGeneralFiles/ProjectFiles/Interfaces/BPI_InteractionInterface.Interact As Target`
  ;[0 0 0] Set Variables
  (if (`self.CanInteract`)
    (set `self.CanInteract` false)
    (set `self.InteractedAsTarget` true)
    (`/Game/MissionsSystem/MissionGeneralFiles/ProjectFiles/Interfaces/BPI_EventInterface.Interact Target Info` (`/Game/MissionsSystem/MissionGeneralFiles/ProjectFiles/Interfaces/BPI_Manager.Get Mission Manager`) (`.MissionActorUniqueName_11_29BEE6AB44E8392C255FDCA7E69E3563` (break `/Game/MissionsSystem/MissionGeneralFiles/ProjectFiles/Structures/ActorStructures/BPS_NPCInfo` (`self.Constructed Actor Info`))))
    (`self.Highlight Actor?` false)
    (set `self.Target?` false)))

(event `/Game/MissionsSystem/MissionGeneralFiles/ProjectFiles/Interfaces/BPI_InteractionInterface.Enable/Disable Actor`
  (params (`Enabled?` :type Boolean) (`Current Mission Index` :type Integer))
  (bind (_overlapmissionactor_ _missionactoruniquename _missionactortype _actorenabled_ _multimissionactorinfo _missionlist) (break `/Game/MissionsSystem/MissionGeneralFiles/ProjectFiles/Structures/ActorStructures/BPS_NPCInfo` (`self.ActorInfo`)))
  (set `self.ActorInfo` (make `/Game/MissionsSystem/MissionGeneralFiles/ProjectFiles/Structures/ActorStructures/BPS_NPCInfo` _overlapmissionactor_ _missionactoruniquename _missionactortype `Enabled?` _multimissionactorinfo _missionlist (make `/Game/MissionsSystem/MissionGeneralFiles/ProjectFiles/Structures/MainStructures/BPS_NonEditNPCInfo` :`Actor Should Be Enabled?` `Enabled?` :`Current Mission Index` `Current Mission Index` :`Self Reference` self)))
  (set `self.MissionAccepted` false)
  (`SceneComponent.SetHiddenInGame` (`self.ParticleSystem`) (not (and `Enabled?` _overlapmissionactor_)) false))

(event `Set Mission Accepted`
  (bind _particlesystem (`self.ParticleSystem`))
  ;[0 0 0] Set Variables
  (`self.Highlight Actor?` false)
  (set `self.MissionAccepted` true)
  (set `self.IsOverlapped` false)
  ;;[0.1302 0 0 1 14] Hide Overlap Mission Actor When Missions Accepted
  (`SceneComponent.SetHiddenInGame` _particlesystem true false)
  (`SceneComponent.SetVisibility` _particlesystem false false))

(event `Set As Target`
  (params (`Target?` :type Boolean))
  ;[0 0 0] Set Variables
  (set `self.Target?` `Target?`))

(event `self.Box.OnComponentBeginOverlap`
  (params (OverlappedComponent :type "PrimitiveComponent Object Reference") (OtherActor :type "Actor Object Reference") (OtherComp :type "PrimitiveComponent Object Reference") (OtherBodyIndex :type Integer) (bFromSweep :type Boolean) (SweepResult :type "HitResult Structure (by ref)"))
  ;[0 0 0] Overlap Events
  (if (`self.Target?`)
    (if (`KismetSystemLibrary.DoesImplementInterface` OtherActor "/Game/MissionsSystem/MissionGeneralFiles/ProjectFiles/Interfaces/BPI_EventInterface.BPI_EventInterface_C")
      (`/Game/MissionsSystem/MissionGeneralFiles/ProjectFiles/Interfaces/BPI_EventInterface.Pass Target Reference` (`/Game/MissionsSystem/MissionGeneralFiles/ProjectFiles/Interfaces/BPI_Manager.Get Mission Manager`) self)
      (`self.Highlight Actor?` true)
      (set `self.IsOverlapped` true))
    (elif (and (`KismetSystemLibrary.DoesImplementInterface` OtherActor "/Game/MissionsSystem/MissionGeneralFiles/ProjectFiles/Interfaces/BPI_EventInterface.BPI_EventInterface_C") (not (`self.MissionAccepted`)) (`.ActorShouldBeEnabled?_10_7282394445A0A0AE401ED4962D93A8C9` (break `/Game/MissionsSystem/MissionGeneralFiles/ProjectFiles/Structures/MainStructures/BPS_NonEditNPCInfo` (`.NonEditNPCInfo_37_E9A04DA043835A0855F3A2B01EF467EA` (break `/Game/MissionsSystem/MissionGeneralFiles/ProjectFiles/Structures/ActorStructures/BPS_NPCInfo` (`self.Constructed Actor Info`))))))
      (`/Game/MissionsSystem/MissionGeneralFiles/ProjectFiles/Interfaces/BPI_EventInterface.Pass NPC Reference` (`/Game/MissionsSystem/MissionGeneralFiles/ProjectFiles/Interfaces/BPI_Manager.Get Mission Manager`) self)
      (if (`self.Has Enough Mission?` true)
        (if (`.OverlapMissionActor?_8_A2E407AB4B0A03B94C6FFFB1D7218F89` (break `/Game/MissionsSystem/MissionGeneralFiles/ProjectFiles/Structures/ActorStructures/BPS_NPCInfo` (`self.Constructed Actor Info`)))
          (message `/Game/MissionsSystem/MissionGeneralFiles/ProjectFiles/Interfaces/BPI_InteractionInterface.Interact With NPC` self)
          (else
            (`self.Highlight Actor?` true)
            (set `self.IsOverlapped` true)))))))

(event `self.Box.OnComponentEndOverlap`
  (params (OverlappedComponent :type "PrimitiveComponent Object Reference") (OtherActor :type "Actor Object Reference") (OtherComp :type "PrimitiveComponent Object Reference") (OtherBodyIndex :type Integer))
  (bind _mission_events (`/Game/MissionsSystem/MissionGeneralFiles/ProjectFiles/Interfaces/BPI_Manager.Get Mission Manager`))
  ;[0 0 0] Overlap Events
  (if (`KismetSystemLibrary.DoesImplementInterface` OtherActor "/Game/MissionsSystem/MissionGeneralFiles/ProjectFiles/Interfaces/BPI_EventInterface.BPI_EventInterface_C")
    (`self.Highlight Actor?` false)
    (set `self.CanInteract` true)
    (set `self.IsOverlapped` false)
    (`/Engine/EditorBlueprintResources/StandardMacros.IsValid` (`KismetSystemLibrary.Conv_InterfaceToObject` _mission_events)
      (:`Is Valid`
        (`/Game/MissionsSystem/MissionGeneralFiles/ProjectFiles/Interfaces/BPI_EventInterface.Remove NPC Reference` _mission_events)))))

(event `/Game/MissionsSystem/MissionGeneralFiles/ProjectFiles/Interfaces/BPI_InteractionInterface.Interact With NPC`
  ;[0 0 0] Interaction With Mission Actor
  (if (`self.CanInteract`)
    (set `self.CanInteract` false)
    (for (_array_element _array_index) (`self.Missions`)
      (bind ((`MissionPanel_117_527A99F94BE3D33563D48EACFEC97CF5` _missionpanel) (`MissionInfo_124_29082C234418A86FE89F17A9F6EC7A0B` _missioninfo) (`OnMissionFinished_128_32275BD648ECA81302C51BBE8EE7AA8E` _onmissionfinished)) (break `/Game/MissionsSystem/MissionGeneralFiles/ProjectFiles/Structures/MainStructures/BPS_MissionMaster` _array_element))
      (`KismetArrayLibrary.Array_Set` (`self.Missions`) _array_index (make `/Game/MissionsSystem/MissionGeneralFiles/ProjectFiles/Structures/MainStructures/BPS_MissionMaster` _missionpanel _missioninfo _onmissionfinished (`.MissionActorUniqueName_11_29BEE6AB44E8392C255FDCA7E69E3563` (break `/Game/MissionsSystem/MissionGeneralFiles/ProjectFiles/Structures/ActorStructures/BPS_NPCInfo` (`self.Constructed Actor Info`))))))
    (`self.Should Show Only One Mission?`
      (:`Return Value`
        (`/Game/MissionsSystem/MissionGeneralFiles/ProjectFiles/Interfaces/BPI_EventInterface.Get Mission Panel` (`/Game/MissionsSystem/MissionGeneralFiles/ProjectFiles/Interfaces/BPI_Manager.Get Mission Manager`) (`self.Constructed Actor Info`))
        (`self.Highlight Actor?` false)))))

(event `Retrigger Overlap Event`
  (params (`Enabled?` :type Boolean))
  (set `self.CanInteract` `Enabled?`)
  (`self.Highlight Actor?` `Enabled?`))

(event `/Game/MissionsSystem/MissionGeneralFiles/ProjectFiles/Interfaces/BPI_InteractionInterface.On Mission Start`
  (bind _asbp_mission_component (cast `/Game/MissionsSystem/MissionGeneralFiles/ProjectFiles/Blueprints/Player/BP_Mission_Component` (`/Game/MissionsSystem/MissionGeneralFiles/ProjectFiles/Interfaces/BPI_Manager.Get Mission Manager`)))
  (add `/Game/MissionsSystem/MissionGeneralFiles/ProjectFiles/Blueprints/Player/BP_Mission_Component.OnFinish` _asbp_mission_component (delegate `OnFinishMision`)))

(event `OnFinishMision`)

(event `self.ReceiveBeginPlay`
  (`KismetSystemLibrary.Delay` 0.2)
  (`/Game/MissionsSystem/MissionGeneralFiles/ProjectFiles/Interfaces/BPI_ObjectivesInterface.Assign NPCs` (`/Game/MissionsSystem/MissionGeneralFiles/ProjectFiles/Interfaces/BPI_Manager.Get Objective Manager`) (`self.Constructed Actor Info`))
  (bind _outactors (`GameplayStatics.GetAllActorsOfClass` "/Script/Engine.TargetPoint"))
  (for _array_element _outactors
    (switch `name` (`|GetArrayItem` (`Actor.Tags` _array_element))
      (:`Mission2`
        (set `self.Mission2` _array_element))
      (:`Mission3`
        (set `self.Mission3` _array_element))
      (:`Mission4`
        (set `self.Mission4` _array_element))
      (:`Mission5`
        (set `self.Mission5` _array_element)))))

(event `self.ReceiveEndPlay`
  (params (EndPlayReason :type "EEndPlayReason Enum" :default "Destroyed"))
  (bind _objective (`/Game/MissionsSystem/MissionGeneralFiles/ProjectFiles/Interfaces/BPI_Manager.Get Objective Manager`))
  (switch `EEndPlayReason` EndPlayReason
    (:`Destroyed`
      _)
    (:`RemovedFromWorld`
      _))
  (`/Engine/EditorBlueprintResources/StandardMacros.IsValid` (`KismetSystemLibrary.Conv_InterfaceToObject` _objective)
    (:`Is Valid`
      (`/Game/MissionsSystem/MissionGeneralFiles/ProjectFiles/Interfaces/BPI_ObjectivesInterface.Remove NPCs` _objective (`self.ActorInfo`)))))

(fn `Add Mission List To Array`
  (bind ((`MissionList_7_EB9DF8684FDEF22D23DB9DBD1E783FBC` _missionlist)) (break `/Game/MissionsSystem/MissionGeneralFiles/ProjectFiles/Structures/ActorStructures/BPS_NPCInfo` (`self.ActorInfo`)))
  (bind _outrownames (`DataTableFunctionLibrary.GetDataTableRowNames` _missionlist))
  (for _array_element _outrownames
    (bind _returnvalue (`|GetDataTableRow` _missionlist _array_element)
      (:`then`
        (`KismetArrayLibrary.Array_Add` (`self.Missions`) _returnvalue))
      (:`RowNotFound`
        (`self.Debug` 4.0 "Mission Data Table Row Not Found. If You Have Already Added One, Please Try To Refresh Actor."))))
  (return))

(fn `Constructed Actor Info`
  (returns (`Constructed Actor Info` :type "/Game/MissionsSystem/MissionGeneralFiles/ProjectFiles/Structures/ActorStructures/BPS_NPCInfo Structure"))
  (bind (_overlapmissionactor_ _missionactoruniquename _missionactortype _actorenabled_ _multimissionactorinfo _missionlist _noneditnpcinfo) (break `/Game/MissionsSystem/MissionGeneralFiles/ProjectFiles/Structures/ActorStructures/BPS_NPCInfo` (`self.ActorInfo`)))
  (bind (_actorshouldbeenabled_ _currentmissionindex) (break `/Game/MissionsSystem/MissionGeneralFiles/ProjectFiles/Structures/MainStructures/BPS_NonEditNPCInfo` _noneditnpcinfo))
  (return (make `/Game/MissionsSystem/MissionGeneralFiles/ProjectFiles/Structures/ActorStructures/BPS_NPCInfo` _overlapmissionactor_ _missionactoruniquename _missionactortype _actorenabled_ _multimissionactorinfo _missionlist (make `/Game/MissionsSystem/MissionGeneralFiles/ProjectFiles/Structures/MainStructures/BPS_NonEditNPCInfo` _actorshouldbeenabled_ _currentmissionindex (`self.Missions`) self))))

(fn `Has Enough Mission?`
  (params (`Check Enabled?` :type Boolean))
  (returns (ReturnValue :type Boolean))
  (bind _missions (`self.Missions`))
  (return (and (select `bool` (`.MultiMissionActor?_5_2398B175431C2F8FAC552196AC76B898` (break `/Game/MissionsSystem/MissionGeneralFiles/ProjectFiles/Structures/OptionStructures/BPS_MultiMissionActorInfo` (`.MultiMissionActorInfo_22_C0E0827D46687A3D31AE409C5D41E677` (break `/Game/MissionsSystem/MissionGeneralFiles/ProjectFiles/Structures/ActorStructures/BPS_NPCInfo` (`self.ActorInfo`))))) :`false` (<= (`self.MissionIndex`) (`KismetArrayLibrary.Array_LastIndex` _missions)) :`true` (>= (`KismetArrayLibrary.Array_Length` _missions) 1)) (select `bool` `Check Enabled?` :`false` true :`true` (`.ActorShouldBeEnabled?_10_7282394445A0A0AE401ED4962D93A8C9` (break `/Game/MissionsSystem/MissionGeneralFiles/ProjectFiles/Structures/MainStructures/BPS_NonEditNPCInfo` (`.NonEditNPCInfo_37_E9A04DA043835A0855F3A2B01EF467EA` (break `/Game/MissionsSystem/MissionGeneralFiles/ProjectFiles/Structures/ActorStructures/BPS_NPCInfo` (`self.Constructed Actor Info`)))))) (not (`self.MissionAccepted`)))))

(fn `UserConstructionScript`
  (bind _interactiondistance (`self.InteractionDistance`))
  (bind _mesh (`self.Mesh`))
  (bind _mesh_2 (`self.Mesh`))
  (bind _particlesystem (`self.ParticleSystem`))
  (`self.Refresh Construction`)
  (`self.Add Mission List To Array`)
  (`BoxComponent.SetBoxExtent` (`self.Box`) (`KismetMathLibrary.MakeVector` _interactiondistance _interactiondistance 70.0) true)
  (`PrimitiveComponent.SetCollisionEnabled` (`self.ParticleSystem`) "NoCollision")
  (if (`.OverlapMissionActor?_8_A2E407AB4B0A03B94C6FFFB1D7218F89` (break `/Game/MissionsSystem/MissionGeneralFiles/ProjectFiles/Structures/ActorStructures/BPS_NPCInfo` (`self.Constructed Actor Info`)))
    (`SceneComponent.SetVisibility` _mesh false true)
    (`PrimitiveComponent.SetCollisionResponseToChannel` (`self.CapsuleComponent`) "ECC_Pawn" "ECR_Overlap")
    (`PrimitiveComponent.SetCollisionResponseToChannel` _mesh "ECC_Pawn" "ECR_Overlap")
    (`PrimitiveComponent.SetCollisionResponseToChannel` _mesh "ECC_Camera" "ECR_Overlap")
    (`PrimitiveComponent.SetCollisionResponseToChannel` (`self.CapsuleComponent`) "ECC_Camera" "ECR_Overlap")
    (`SceneComponent.SetVisibility` (`self.ParticleSystem`) true true)
    (if (`self.Has Enough Mission?` true)
      (`SceneComponent.SetHiddenInGame` _particlesystem false true)
      (else
        (`SceneComponent.SetHiddenInGame` _particlesystem true true)))
    (else
      (`SceneComponent.SetVisibility` (`self.ParticleSystem`) false true)
      (`SceneComponent.SetVisibility` _mesh_2 true true)
      (`PrimitiveComponent.SetCollisionResponseToChannel` _mesh_2 "ECC_Pawn" "ECR_Block")
      (`PrimitiveComponent.SetCollisionResponseToChannel` (`self.CapsuleComponent`) "ECC_Pawn" "ECR_Block")
      (`PrimitiveComponent.SetCollisionResponseToChannel` (`self.CapsuleComponent`) "ECC_Camera" "ECR_Block")
      (`PrimitiveComponent.SetCollisionResponseToChannel` _mesh_2 "ECC_Camera" "ECR_Block"))))