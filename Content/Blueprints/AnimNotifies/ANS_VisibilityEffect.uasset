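; Anim notify state that drives a mesh's material visibility from an animation curve, such as for a spawn effect.
; Each tick it reads the "Spawn" curve from the mesh's anim instance and writes it to the "Visibility" scalar parameter on all materials.
; On end it applies the curve value once more so the materials keep the final value.
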(fn `Received_NotifyEnd`
  (params (MeshComp :type "SkeletalMeshComponent Object Reference") (Animation :type "AnimSequenceBase Object Reference"))
  (returns (ReturnValue :type Boolean))
  (`/Engine/EditorBlueprintResources/StandardMacros.IsValid` MeshComp
    (:`Is Valid`
      (`MeshComponent.SetScalarParameterValueOnMaterials` MeshComp "Visibility" (`AnimInstance.GetCurveValue` (`SkeletalMeshComponent.GetAnimInstance` MeshComp) "Spawn"))
      (return true))))

(fn `Received_NotifyTick`
  (params (MeshComp :type "SkeletalMeshComponent Object Reference") (Animation :type "AnimSequenceBase Object Reference") (FrameDeltaTime :type "Float (double-precision)"))
  (returns (ReturnValue :type Boolean))
  (`/Engine/EditorBlueprintResources/StandardMacros.IsValid` MeshComp
    (:`Is Valid`
      (`MeshComponent.SetScalarParameterValueOnMaterials` MeshComp "Visibility" (`AnimInstance.GetCurveValue` (`SkeletalMeshComponent.GetAnimInstance` MeshComp) "Spawn"))
      (return true))))