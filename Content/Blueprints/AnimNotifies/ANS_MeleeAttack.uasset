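; Anim notify state that marks the active attack window of a melee animation for player characters and enemies.
; On begin, it resolves the owner's weapon, from the player's equipped slot or the enemy's current weapon, flags it as attacking and starts its attack with an event tag and delay settings.
; On end, it resolves the weapon again and ends the attack.
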(fn `Received_NotifyBegin`
  (params (MeshComp :type "SkeletalMeshComponent Object Reference") (Animation :type "AnimSequenceBase Object Reference") (TotalDuration :type "Float (double-precision)"))
  (returns (ReturnValue :type Boolean))
  (locals (WeaponActor :type "/Game/Blueprints/Weapon/BP_WeaponActor Object Reference"))
  (bind _returnvalue (`ActorComponent.GetOwner` MeshComp))
  (bind _asbp_player_character (cast `/Game/Blueprints/BP_PlayerCharacter` _returnvalue)
    (:`then`
      (set `local.WeaponActor` (cast `/Game/Blueprints/Weapon/BP_WeaponActor` (`BlueprintMapLibrary.Map_Find` (`/Game/Blueprints/BP_PlayerCharacter.EquippedWeapons` _asbp_player_character) (`self.SlotWeapon`)) :!pure true)))
    (:`CastFailed`
      (bind _asbp_enemy_base (cast `/Game/Blueprints/NPC/Enemies/BP_EnemyBase` _returnvalue))
      (set `local.WeaponActor` (`/Game/Blueprints/NPC/Enemies/BP_EnemyBase.CurrentWeapon` _asbp_enemy_base))))
  (bind _weaponactor (`local.WeaponActor`)
    (:`then`
      (set `/Game/Blueprints/Weapon/BP_WeaponActor.bIsAttacking` true _weaponactor)
      (`/Game/Blueprints/Weapon/BP_WeaponActor.BeginWeaponAttack` _weaponactor (`self.EventTag`) (`self.AttackDelayTime`) (`self.MaxAttackDelayCount`))
      (return true))
    (:`else`)))

(fn `Received_NotifyEnd`
  (params (MeshComp :type "SkeletalMeshComponent Object Reference") (Animation :type "AnimSequenceBase Object Reference"))
  (returns (ReturnValue :type Boolean))
  (locals (WeaponActor :type "/Game/Blueprints/Weapon/BP_WeaponActor Object Reference"))
  (bind _returnvalue (`ActorComponent.GetOwner` MeshComp))
  (bind _asbp_player_character (cast `/Game/Blueprints/BP_PlayerCharacter` _returnvalue)
    (:`then`
      (set `local.WeaponActor` (cast `/Game/Blueprints/Weapon/BP_WeaponActor` (`BlueprintMapLibrary.Map_Find` (`/Game/Blueprints/BP_PlayerCharacter.EquippedWeapons` _asbp_player_character) (`self.SlotWeapon`)) :!pure true)))
    (:`CastFailed`
      (bind _asbp_enemy_base (cast `/Game/Blueprints/NPC/Enemies/BP_EnemyBase` _returnvalue))
      (set `local.WeaponActor` (`/Game/Blueprints/NPC/Enemies/BP_EnemyBase.CurrentWeapon` _asbp_enemy_base))))
  (bind _weaponactor (`local.WeaponActor`)
    (:`then`
      (`/Game/Blueprints/Weapon/BP_WeaponActor.EndWeaponAttack` _weaponactor)
      (return false))
    (:`else`)))