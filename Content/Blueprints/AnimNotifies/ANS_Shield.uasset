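; Anim notify state that makes a shielded player character immune for the duration of a marked animation window.
; Notify begin applies the ShieldGE gameplay effect to the owning BP_PlayerCharacter's ability system when IsProtectedByShield is set.
; Notify end removes all stacks of that effect, but only if the shield flag is still set at that moment.
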(fn `Received_NotifyBegin`
  (params (MeshComp :type "SkeletalMeshComponent Object Reference") (Animation :type "AnimSequenceBase Object Reference") (TotalDuration :type "Float (double-precision)"))
  (returns (ReturnValue :type Boolean))
  (bind _asbp_player_character (cast `/Game/Blueprints/BP_PlayerCharacter` (`ActorComponent.GetOwner` MeshComp)))
  (if (`/Game/Blueprints/BP_PlayerCharacter.bIsProtectedByShield` _asbp_player_character)
    ;[1 1 1] Apply immunity effect
    (`AbilitySystemComponent.BP_ApplyGameplayEffectToSelf` :`self` (`AbilitySystemBlueprintLibrary.GetAbilitySystemComponent` _asbp_player_character) :`GameplayEffectClass` (`self.ShieldGE`))
    (return true)))

(fn `Received_NotifyEnd`
  (params (MeshComp :type "SkeletalMeshComponent Object Reference") (Animation :type "AnimSequenceBase Object Reference"))
  (returns (ReturnValue :type Boolean))
  (bind _asbp_player_character (cast `/Game/Blueprints/BP_PlayerCharacter` (`ActorComponent.GetOwner` MeshComp)))
  (if (`/Game/Blueprints/BP_PlayerCharacter.bIsProtectedByShield` _asbp_player_character)
    ;[1 1 1] Removed immunity added in begin
    (`AbilitySystemComponent.RemoveActiveGameplayEffectBySourceEffect` (`AbilitySystemBlueprintLibrary.GetAbilitySystemComponent` _asbp_player_character) (`self.ShieldGE`) null -1)
    (return true)))