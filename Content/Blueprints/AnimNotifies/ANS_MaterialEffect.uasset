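; ANS_MaterialEffect is an anim notify state that toggles a colored material effect on the animated mesh for the duration of the notify window.
; On begin it writes its LinearColor value to the EffectColor vector parameter and sets the Target_Switch_On scalar to turn the effect on.
; On end it writes the same color again and zeroes the switch, relying on the mesh's materials exposing both parameters.
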(fn `Received_NotifyBegin`
  (params (MeshComp :type "SkeletalMeshComponent Object Reference") (Animation :type "AnimSequenceBase Object Reference") (TotalDuration :type "Float (double-precision)"))
  (returns (ReturnValue :type Boolean))
  (`MeshComponent.SetVectorParameterValueOnMaterials` MeshComp "EffectColor" (`KismetMathLibrary.Conv_LinearColorToVector` (`self.LinearColor`)))
  (`MeshComponent.SetScalarParameterValueOnMaterials` MeshComp "Target_Switch_On" (`self.01`))
  (return true))

(fn `Received_NotifyEnd`
  (params (MeshComp :type "SkeletalMeshComponent Object Reference") (Animation :type "AnimSequenceBase Object Reference"))
  (returns (ReturnValue :type Boolean))
  (`MeshComponent.SetVectorParameterValueOnMaterials` MeshComp "EffectColor" (`KismetMathLibrary.Conv_LinearColorToVector` (`self.LinearColor`)))
  (`MeshComponent.SetScalarParameterValueOnMaterials` MeshComp "Target_Switch_On" (`self.00`))
  (return false))