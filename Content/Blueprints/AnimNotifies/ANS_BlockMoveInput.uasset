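; Animation notify state that blocks the player character's movement input for the span it covers in an animation.
; On begin, with a valid mesh, it sets BlockedMovementInput on the PlayerCharacter reached through the player controller, and on end it clears the flag if that controller is valid.
; The target is the controller's character, not the owner of the animated mesh.
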(fn `Received_NotifyBegin`
  (params (MeshComp :type "SkeletalMeshComponent Object Reference") (Animation :type "AnimSequenceBase Object Reference") (TotalDuration :type "Float (double-precision)"))
  (returns (ReturnValue :type Boolean))
  (`/Engine/EditorBlueprintResources/StandardMacros.IsValid` MeshComp
    (:`Is Valid`
      (bind _output_get (set `EdenValleyCharacterBaseMainActor.bBlockedMovementInput` true (`/Game/Blueprints/BP_PlayerController.PlayerCharacter` (`/Game/Blueprints/BP_FunctionLibrary.GetPlayerControllerBP` MeshComp))))
      (return _output_get))))

(fn `Received_NotifyEnd`
  (params (MeshComp :type "SkeletalMeshComponent Object Reference") (Animation :type "AnimSequenceBase Object Reference"))
  (returns (ReturnValue :type Boolean))
  (bind _playercontroller (`/Game/Blueprints/BP_FunctionLibrary.GetPlayerControllerBP` MeshComp))
  (`/Engine/EditorBlueprintResources/StandardMacros.IsValid` _playercontroller
    (:`Is Valid`
      (bind _output_get (set `EdenValleyCharacterBaseMainActor.bBlockedMovementInput` false (`/Game/Blueprints/BP_PlayerController.PlayerCharacter` _playercontroller)))
      (return _output_get))))