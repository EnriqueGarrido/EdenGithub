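; BP_Soul is a short-lived soul actor that rises into the air and then removes itself.
; After a brief random delay on BeginPlay, it turns off physics simulation on its Sphere and records its current location.
; The MoveToSky timeline then lerps the actor straight up by a fixed height without sweeping, and destroys it when finished.
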(event `self.ReceiveBeginPlay`
  (`KismetSystemLibrary.Delay` (`KismetMathLibrary.RandomFloatInRange` 0.5 1.0))
  (`PrimitiveComponent.SetSimulatePhysics` (`self.Sphere`) false)
  (set `self.InitialActorLocation` (`self.K2_GetActorLocation`))
  (bind (_direction _alpha) (`Timeline|MoveToSky`)
    (:`Update`
      (`self.K2_SetActorLocation` (`KismetMathLibrary.VLerp` (`self.InitialActorLocation`) (`KismetMathLibrary.MakeVector` (.x (`self.InitialActorLocation`)) (.y (`self.InitialActorLocation`)) (+ (.z (`self.InitialActorLocation`)) 200.0)) _alpha)))
    (:`Finished`
      (`self.K2_DestroyActor`))))

(fn `UserConstructionScript`)