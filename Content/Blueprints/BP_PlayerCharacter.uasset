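; Player character Blueprint for an action RPG, handling combat, equipment, interaction and mission input.
; Input triggers Gameplay Ability System abilities by item slot or class, with gameplay events stopping defense and passing overlapped enemies to magic damage.
; Equipped items spawn weapon actors from a data table onto sockets, gating shield and skill use.
; Attribute changes update the HUD and death, while the mission manager drives markers, compass and sequence skipping.
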(event `InputAxis|Turn` :overrideparent false
  (params (AxisValue :type "Float (single-precision)"))
  (if (!= AxisValue 0.0)
    (`/Game/MissionsSystem/MissionGeneralFiles/ProjectFiles/Interfaces/BPI_EventInterface.Update Compass And Markers` (`/Game/MissionsSystem/MissionGeneralFiles/ProjectFiles/Interfaces/BPI_Manager.Get Mission Manager`))))

(event `InputAction|Talk`
  (params (Key :type "Key Structure"))
  (:`Pressed`
    (`/Game/MissionsSystem/MissionGeneralFiles/ProjectFiles/Interfaces/BPI_EventInterface.Accept Mission` (`/Game/MissionsSystem/MissionGeneralFiles/ProjectFiles/Interfaces/BPI_Manager.Get Mission Manager`))))

(event `self.OnMoveForward`
  (params (Value :type "Float (single-precision)"))
  (`/Game/MissionsSystem/MissionGeneralFiles/ProjectFiles/Interfaces/BPI_EventInterface.Update Compass And Markers` (`/Game/MissionsSystem/MissionGeneralFiles/ProjectFiles/Interfaces/BPI_Manager.Get Mission Manager`)))

(event `self.OnMoveRight`
  (params (Value :type "Float (single-precision)"))
  (`/Game/MissionsSystem/MissionGeneralFiles/ProjectFiles/Interfaces/BPI_EventInterface.Update Compass And Markers` (`/Game/MissionsSystem/MissionGeneralFiles/ProjectFiles/Interfaces/BPI_Manager.Get Mission Manager`)))

(event `Key|Tab`
  (params (Key :type "Key Structure")))

(event `InputAction|Jump` :paused true :overrideparent false
  (params (Key :type "Key Structure"))
  (bind _mission_component (`self.Mission Component`))
  (bind _sequenceplaying_ (`/Game/MissionsSystem/MissionGeneralFiles/ProjectFiles/Blueprints/Player/BP_Mission_Component.SequencePlaying?` _mission_component))
  (bind _missionpanel (`/Game/MissionsSystem/MissionGeneralFiles/ProjectFiles/UI/UI_HUD_Layout2.MissionPanel` (`/Game/MissionsSystem/MissionGeneralFiles/ProjectFiles/Blueprints/Player/BP_Mission_Component.HUDReference` _mission_component)))
  (:`Pressed`
    (if (not (or _sequenceplaying_ (`/Game/MissionsSystem/MissionGeneralFiles/ProjectFiles/Blueprints/Player/BP_Mission_Component.CurrentMissionsOpened` _mission_component) (or (`/Game/MissionsSystem/MissionGeneralFiles/ProjectFiles/UI/Missions/Main/UI_MissionPanel.MultiOpened?` _missionpanel) (`/Game/MissionsSystem/MissionGeneralFiles/ProjectFiles/UI/Missions/Main/UI_MissionPanel.SingleOpened?` _missionpanel))))
      (`self.Jump`)
      (else
        (`self.StopJumping`)
        (if _sequenceplaying_
          (`/Game/MissionsSystem/MissionGeneralFiles/ProjectFiles/Interfaces/BPI_EventInterface.Skip Sequence` (`/Game/MissionsSystem/MissionGeneralFiles/ProjectFiles/Interfaces/BPI_Manager.Get Mission Manager`) Key)))))
  (:`Released`
    (`self.StopJumping`)))

(event `ShowAllNPCMarkers`
  (bind _mission_component (`self.Mission Component`))
  (for _array_element (`/Game/MissionsSystem/MissionGeneralFiles/ProjectFiles/Blueprints/Player/BP_Mission_Component.DefaultMissionMarkers` _mission_component)
    (bind (_displaymarkeronscreen_ _npcuniquename _nearestlocationforlevelstreaming _customizemarker) (break `/Game/MissionsSystem/MissionGeneralFiles/ProjectFiles/Structures/MainStructures/BPS_NPCMarkersInfo` _array_element))
    (`/Game/MissionsSystem/MissionGeneralFiles/ProjectFiles/Blueprints/Player/BP_Mission_Component.AddNPCMarkersToScreen` _mission_component (make `/Game/MissionsSystem/MissionGeneralFiles/ProjectFiles/Structures/MainStructures/BPS_NPCMarkersInfo` true _npcuniquename _nearestlocationforlevelstreaming _customizemarker))))

(event `self.ReceiveBeginPlay`
  ;[0 0 0] Missions setup
  (`/Game/MissionsSystem/MissionGeneralFiles/ProjectFiles/Interfaces/BPI_EventInterface.Create Mission UI` (`/Game/MissionsSystem/MissionGeneralFiles/ProjectFiles/Interfaces/BPI_Manager.Get Mission Manager`) self (`self.FollowCamera`))
  (bind _loadmissions (`/Game/Blueprints/BP_GameInstance.GetLoadMission` (`/Game/Blueprints/BP_FunctionLibrary.GetGameInstanceBP`)))
  (`KismetArrayLibrary.Array_Add` (`/Game/MissionsSystem/MissionGeneralFiles/ProjectFiles/Blueprints/Player/BP_Mission_Component.DefaultMissionMarkers` (`self.Mission Component`)) (make `/Game/MissionsSystem/MissionGeneralFiles/ProjectFiles/Structures/MainStructures/BPS_NPCMarkersInfo` false (break `/Game/Blueprints/SaveGame/LoadMissionsStruct` _loadmissions) (0.0 0.0 0.0) (make `/Game/MissionsSystem/MissionGeneralFiles/ProjectFiles/Structures/MainStructures/BPS_CustomMarker` false true (struct :`R` 1.0 :`G` 1.0 :`B` 1.0 :`A` 0.8) (struct :`R` 1.0 :`G` 1.0 :`B` 1.0 :`A` 1.0) "/Game/MissionsSystem/MissionGeneralFiles/ProjectFiles/Materials/Compass/Markers/MI_Marker1.MI_Marker1"))))

(event `InputAction|Attack`
  (params (Key :type "Key Structure"))
  ;[1 1 1] Handle input
  (:`Pressed`
    (if (`self.bIsTargeting`)
      (`AbilitySystemComponent.TargetConfirm` (`AbilitySystemBlueprintLibrary.GetAbilitySystemComponent` self))
      (set `self.bIsTargeting` false)
      (else
        (`self.MeleeAttack`)))))

(event `InputAction|UsePotion`
  (params (Key :type "Key Structure"))
  ;[1 1 1] Handle input
  (:`Pressed`
    (`self.UsePotion`)))

(event `InputAction|UseSkill`
  (params (Key :type "Key Structure"))
  ;[1 1 1] Handle input
  (:`Pressed`
    (`self.Use skill`)))

(event `InputAction|Roll`
  (params (Key :type "Key Structure"))
  ;[1 1 1] Handle input
  (:`Pressed`
    (`self.DoRoll`)))

(event `InputAction|Shield`
  (params (Key :type "Key Structure"))
  ;[1 1 1] Handle input
  (:`Pressed`
    (`self.DefendShield`))
  (:`Released`
    (`self.StopShield`)))

(event `InputAction|Interact`
  (params (Key :type "Key Structure"))
  ;[1 1 1] Handle input
  (:`Pressed`
    (`self.HandleInteraction`)))

(event `self.OnHealthChanged`
  (params (HealthAmount :type "Float (single-precision)") (EventTags :type "GameplayTagContainer Structure (by ref)"))
  ;[1 1 1] Handle changes
  (`self.UpdateHealth`)
  (bind _returnvalue (`self.IsAlive`))
  (if (not _returnvalue)
    (`/Engine/EditorBlueprintResources/StandardMacros.DoOnce` false
      (:`Completed`
        (bind _returnvalue_2 (`self.PlayAnimMontage` "/Game/Characters/Animations/NoWeaponStance/AM_Die_noWeaponAnim_Montage.AM_Die_noWeaponAnim_Montage"))
        (`KismetSystemLibrary.Delay` _returnvalue_2)))))

(event `OnDeathEvent`
  ;[1 1 1] Called when character is dying
  (`/Engine/EditorBlueprintResources/StandardMacros.IsValid` (`self.Mission Component`)
    (:`Is Valid`
      (`Widget.RemoveFromParent` (`/Game/MissionsSystem/MissionGeneralFiles/ProjectFiles/Blueprints/Player/BP_Mission_Component.HUDReference` (`self.Mission Component`))))
    (:`Is Not Valid`
      _))
  (`/Game/Blueprints/BP_GameModeBase.GameOver` (`/Game/Blueprints/BP_FunctionLibrary.GetGameModeBP`)))

(event `self.OnManaChanged`
  (params (ManaAmount :type "Float (single-precision)") (EventTags :type "GameplayTagContainer Structure (by ref)"))
  ;[1 1 1] Handle changes
  (`self.Update Mana`))

(event `self.OnDamageChanged`
  (params (DamageAmount :type "Float (single-precision)") (HitInfo :type "HitResult Structure (by ref)") (DamageTags :type "GameplayTagContainer Structure (by ref)") (InstigatorCharacter :type "EdenValleyCharacterBase Object Reference") (DamageCauser :type "Actor Object Reference"))
  ;[1 1 1] Handle changes
  (`self.DamageChanged`))

(event `MeleeAttack`
  ;[1 1 1] Melee Attack
  (bind _returnvalue (`self.CanUseAnyAbililty`))
  (if _returnvalue
    (bind _returnvalue_2 (`self.ActivateAbilitiesWithItemSlot` 1 true))
    (if _returnvalue_2
      (`self.AbilityDelegate`))))

(event `DoRoll`
  ;[1 1 1] Do roll
  (bind _returnvalue (`self.CanUseAnyAbililty`))
  (if (and _returnvalue (> (`KismetMathLibrary.VSize` (`self.GetVelocity`)) 0.0) (not (`self.bBlockAbilities`)))
    (bind _returnvalue_2 (`AbilitySystemComponent.TryActivateAbilityByClass` (`AbilitySystemBlueprintLibrary.GetAbilitySystemComponent` self) "/Game/Abilities/Player/Roll/GA_Roll.GA_Roll_C" true))
    (if _returnvalue_2
      (`self.AbilityDelegate`))))

(event `UpdateHealth`
  ;[1 1 1] Update Health
  (bind _aswb_hud_character (cast `/Game/Blueprints/UI/HUD/WB_HUD_Character` (`/Game/Blueprints/BP_PlayerController.OnScreenControls` (`/Game/Blueprints/BP_FunctionLibrary.GetPlayerControllerBP`))))
  (`/Game/Blueprints/UI/HUD/WB_HUD_Character.SetHealthProgress` _aswb_hud_character (/ (`self.GetHealth`) (`self.GetMaxHealth`))))

(event `Update Mana`
  ;[1 1 1] Update Mana
  (bind _aswb_hud_character (cast `/Game/Blueprints/UI/HUD/WB_HUD_Character` (`/Game/Blueprints/BP_PlayerController.OnScreenControls` (`/Game/Blueprints/BP_FunctionLibrary.GetPlayerControllerBP`))))
  (`/Game/Blueprints/UI/HUD/WB_HUD_Character.SetManaProgress` _aswb_hud_character (/ (`self.GetMana`) (`self.GetMaxMana`))))

(event `DamageChanged`
  ;[1 1 1] Play animation when the character takes damage
  (bind _returnvalue (`self.CanUseAnyAbililty`))
  (if _returnvalue
    (`self.PlayAnimMontage` "/Game/Characters/Animations/NoWeaponStance/AM_Shield_GetHit.AM_Shield_GetHit")))

(event `UsePotion`
  ;[1 1 1] Use potion added on a slot item
  (bind _returnvalue (`self.CanUseAnyAbililty`))
  (if _returnvalue
    (bind _returnvalue_2 (`self.ActivateAbilitiesWithItemSlot` 4 true))
    (if _returnvalue_2
      (`self.AbilityDelegate`)
      (`self.SkillDelegate`))))

(event `Use skill`
  ;[1 1 1] Use any skill added on a slot item
  (bind _returnvalue (`self.CanUseAnyAbililty`))
  (if (and _returnvalue (`self.bIsSwordAttached`))
    (bind _returnvalue_2 (`self.ActivateAbilitiesWithItemSlot` 3 true))
    (if _returnvalue_2
      (`self.AbilityDelegate`)
      (`self.SkillDelegate`))))

(event `EndCombo`
  ;[1 1 1] End Combo
  (set `self.ComboCount` 1))

(event `self.CapsuleComponent.OnComponentBeginOverlap`
  (params (OverlappedComponent :type "PrimitiveComponent Object Reference") (OtherActor :type "Actor Object Reference") (OtherComp :type "PrimitiveComponent Object Reference") (OtherBodyIndex :type Integer) (bFromSweep :type Boolean) (SweepResult :type "HitResult Structure (by ref)"))
  ;[1 1 1] Handle dashing ability
  (if (`KismetMathLibrary.ClassIsChildOf` (`GameplayStatics.GetObjectClass` OtherActor) "/Game/Blueprints/NPC/Enemies/BP_EnemyBase.BP_EnemyBase_C")
    (`AbilitySystemBlueprintLibrary.SendGameplayEventToActor` self (struct :`TagName` "Skill.Magic.DealDamage") (make `GameplayEventData` (struct) null OtherActor))))

(event `DefendShield`
  ;[1 1 1] Defend
  (if (`self.bIsTargeting`)
    (`AbilitySystemComponent.TargetCancel` (`AbilitySystemBlueprintLibrary.GetAbilitySystemComponent` self))
    (set `self.bIsTargeting` false)
    (else
      (bind _returnvalue (`self.CanUseAnyAbililty`))
      (if (and _returnvalue (`self.bIsProtectedByShield`))
        (bind _returnvalue_2 (`self.ActivateAbilitiesWithItemSlot` 2 true))
        (if _returnvalue_2
          (`self.AbilityDelegate`))))))

(event `StopShield`
  ;[1 1 1] Stop Shield
  (`AbilitySystemBlueprintLibrary.SendGameplayEventToActor` self (struct :`TagName` "Skill.Defend.Stop")))

(event `SwitchWeapon`
  (params (ItemData :type "EdenValleyItemData Object Reference") (SlotNumber :type Integer))
  ;[1 1 1] Switch weapon
  (`self.CreateWeapon` ItemData SlotNumber))

(event `HandleInteraction`
  (bind _currentinteractable (`EdenValleyPlayerController.CurrentInteractable` (`/Game/Blueprints/BP_FunctionLibrary.GetPlayerControllerBP`)))
  ;[1 1 1] Handle interaction of character with item
  (`/Engine/EditorBlueprintResources/StandardMacros.IsValid` _currentinteractable
    (:`Is Valid`
      (`AbilitySystemComponent.TryActivateAbilityByClass` (`AbilitySystemBlueprintLibrary.GetAbilitySystemComponent` self) "/Game/Abilities/Player/PickupItem/GA_PickupItem.GA_PickupItem_C" true)
      (`Interactable.Interact` _currentinteractable (`/Game/Blueprints/BP_FunctionLibrary.GetPlayerControllerBP`)))))

(fn `AttachWeapon`
  (params (SlotNumber :type Integer))
  (locals (SlotToWeapon :type "Map of Integer to Name"))
  (switch `int` SlotNumber
    (:`1`
      (set `self.bIsSwordAttached` true))
    (:`2`
      (set `self.bIsProtectedByShield` true)))
  (`self.K2_AttachToComponent` (`BlueprintMapLibrary.Map_Find` (`self.EquippedWeapons`) (`local.SlotNumber`)) (`self.Mesh`) (`BlueprintMapLibrary.Map_Find` (`local.SlotToWeapon`) (`local.SlotNumber`)) "SnapToTarget" "SnapToTarget" "KeepWorld" true))

(fn `CreateWeapon`
  (params (ItemData :type "EdenValleyItemData Object Reference") (SlotNumber :type Integer))
  (bind _value (`BlueprintMapLibrary.Map_Find` (`self.EquippedWeapons`) (`local.SlotNumber`)))
  ;[1 1 1] Remove weapon and update slots
  (`/Engine/EditorBlueprintResources/StandardMacros.IsValid` ItemData
    (:`Is Valid`
      ;[1 1 1] Attach weapon
      (if (not (`.ReturnValue` (`BlueprintMapLibrary.Map_Find` (`self.EquippedWeapons`) (`local.SlotNumber`))))
        (bind _returnvalue (`|GetDataTableRow` (`EdenValleyGameStateBase.GetWeaponDB` (`/Game/Blueprints/BP_FunctionLibrary.GetGameStateBP`)) (`.ItemID` (break `EdenValleyItem` (`EdenValleyItemData.Item` (`local.ItemData`)))))
          (:`then`
            (bind _returnvalue_2 (`|SpawnActorFromClass` (`.WeaponActor` (break `EdenValleyWeaponItem` _returnvalue)) (`KismetMathLibrary.MakeTransform` (0.0 0.0 -1000.0)) "Undefined" "OverrideRootScale" null null))
            (`BlueprintMapLibrary.Map_Add` (`self.EquippedWeapons`) (`local.SlotNumber`) _returnvalue_2)
            (`self.AttachWeapon` (`local.SlotNumber`))))))
    (:`Is Not Valid`
      (if (not (== _value null))
        (`self.K2_DetachFromActor` _value "KeepRelative" "KeepWorld" "KeepWorld")
        (message `/Game/Blueprints/UI/HUD/iHUD.UpdateSlot` (`/Game/Blueprints/BP_FunctionLibrary.GetPlayerControllerBP`) (`local.SlotNumber`) (`local.ItemData`))
        (bind _returnvalue_3 (`BlueprintMapLibrary.Map_Remove` (`self.EquippedWeapons`) (`local.SlotNumber`)))
        (if _returnvalue_3
          (switch `int` (`local.SlotNumber`)
            (:`1`
              (set `self.bIsSwordAttached` false))
            (:`2`
              (set `self.bIsProtectedByShield` false))))))))

(fn `DetermineCombo`
  (switch `int` (`self.ComboCount`)
    (:`1`
      (set `self.MeleeMontage` "/Game/Characters/Animations/SwordAndShieldStance/AM_Shield_NormalAttack01.AM_Shield_NormalAttack01")
      (`/Engine/EditorBlueprintResources/StandardMacros.IncrementInt` (`self.ComboCount`) :!label _label))
    (:`2`
      (set `self.MeleeMontage` "/Game/Characters/Animations/SwordAndShieldStance/AM_Shield_NormalAttack02.AM_Shield_NormalAttack02")
      (goto _label))
    (:`3`
      (set `self.MeleeMontage` "/Game/Characters/Animations/SwordAndShieldStance/AM_JumpAttack_SwordShieldAnim.AM_JumpAttack_SwordShieldAnim")
      (set `self.ComboCount` 1))))

(fn `SetCollisonToPawn`
  (params (Response :type "ECollisionResponse Enum" :default "ECR_Ignore"))
  (`PrimitiveComponent.SetCollisionResponseToChannel` (`self.CapsuleComponent`) "ECC_Pawn" Response))

(fn `UserConstructionScript`)