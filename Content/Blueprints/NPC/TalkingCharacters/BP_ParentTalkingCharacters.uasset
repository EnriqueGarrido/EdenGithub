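; Parent Blueprint for talking NPCs that shows a Talk indicator while the player overlaps DetectCharacter and runs data-table-driven dialogue.
; BeginPlay caches the table rows matching this NPC's ID.
; CreateDialogue hides the HUD, stops player movement, switches to the talking camera and opens WB_Dialogue.
; GetLineDialogue displays the row matching conversation and line IDs, otherwise restores view, HUD and movement, advancing the conversation when flagged.
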(event `self.ReceiveBeginPlay`
  (`SceneComponent.SetVisibility` (`self.Talk`) false false)
  (bind _asbp_player_character (cast `/Game/Blueprints/BP_PlayerCharacter` (`GameplayStatics.GetPlayerCharacter` 0)))
  (set `self.MainActor` _asbp_player_character)
  (set `self.HUD_Character` (`/Game/Blueprints/BP_PlayerController.OnScreenControls` (`/Game/Blueprints/BP_FunctionLibrary.GetPlayerControllerBP`)))
  (`self.checkIDNPC`))

(event `self.DetectCharacter.OnComponentBeginOverlap`
  (params (OverlappedComponent :type "PrimitiveComponent Object Reference") (OtherActor :type "Actor Object Reference") (OtherComp :type "PrimitiveComponent Object Reference") (OtherBodyIndex :type Integer) (bFromSweep :type Boolean) (SweepResult :type "HitResult Structure (by ref)"))
  ;[1 1 1] Detect when the main actor collision
  (if (== (`GameplayStatics.GetObjectClass` OtherActor) "/Game/Blueprints/BP_PlayerCharacter.BP_PlayerCharacter_C")
    (`SceneComponent.SetVisibility` (`self.Talk`) true false)))

(event `self.DetectCharacter.OnComponentEndOverlap`
  (params (OverlappedComponent :type "PrimitiveComponent Object Reference") (OtherActor :type "Actor Object Reference") (OtherComp :type "PrimitiveComponent Object Reference") (OtherBodyIndex :type Integer))
  ;[1 1 1] Detect when the main actor collision
  (if (== (`GameplayStatics.GetObjectClass` OtherActor) "/Game/Blueprints/BP_PlayerCharacter.BP_PlayerCharacter_C")
    (`SceneComponent.SetVisibility` (`self.Talk`) false false)))

(fn `changeConversation`
  (`/Engine/EditorBlueprintResources/StandardMacros.IncrementInt` (`self.Conversation_ID`)))

(fn `checkIDNPC`
  (bind _outrownames (`DataTableFunctionLibrary.GetDataTableRowNames` "/Game/Data/Dialogue.Dialogue"))
  (for _array_element _outrownames
    (bind _returnvalue (`|GetDataTableRow` "/Game/Data/Dialogue.Dialogue" _array_element)
      (:`then`
        (if (== (`.NPC_ID_3_7A57F537438C4D6600E09AB308CFB4AB` (break `/Game/Blueprints/Dialogue/STRUCT_Dialogue` _returnvalue)) (`self.NPC_ID`))
          (`KismetArrayLibrary.Array_Add` (`self.MyDialogue`) _array_element))))))

(fn `createDialogue`
  (`Widget.SetVisibility` (`self.HUD_Character`) "Hidden")
  (`SceneComponent.SetVisibility` (`self.Talk`) false false)
  (`ActorComponent.Deactivate` (`Character.CharacterMovement` (`self.MainActor`)))
  (`PlayerController.SetViewTargetWithBlend` (`GameplayStatics.GetPlayerController` 0) (`ActorComponent.GetOwner` (`self.TalkingCamera`)) 0.0 "VTBlend_Linear" 0.0 false)
  (bind _returnvalue (`|CreateWidget` "/Game/Blueprints/UI/Dialogue/WB_Dialogue.WB_Dialogue_C" (`GameplayStatics.GetPlayerController` 0) (`self.Avatar`) (`self.inCharge`)))
  (`UserWidget.AddToViewport` _returnvalue 0)
  (set `self.dialogue` _returnvalue)
  (`self.K2_SetActorRotation` (`self.MainActor`) (`KismetMathLibrary.NormalizedDeltaRotator` (`SceneComponent.RelativeRotation` (`self.CapsuleComponent`)) (struct :`Yaw` 180.0)) false)
  (`self.getLineDialogue`))

(fn `getLineDialogue`
  (locals (ReturnedLines :type "Array of Text"))
  (for _array_element (`self.MyDialogue`)
    (bind _returnvalue (`|GetDataTableRow` "/Game/Data/Dialogue.Dialogue" _array_element)
      (:`then`
        (bind (_npc_id _conversation_id _line_id _dialogue _nextconversation) (break `/Game/Blueprints/Dialogue/STRUCT_Dialogue` _returnvalue))
        (if (and (== _conversation_id (`self.Conversation_ID`)) (== _line_id (`self.LineCurrent`)))
          (`KismetArrayLibrary.Array_Add` (`local.ReturnedLines`) _dialogue)
          (set `self.hasNext` _nextconversation)))))
  (if (== (`KismetArrayLibrary.Array_Length` (`local.ReturnedLines`)) 1)
    (bind _aswb_dialogue (cast `/Game/Blueprints/UI/Dialogue/WB_Dialogue` (`self.dialogue`)))
    (set `/Game/Blueprints/UI/Dialogue/WB_Dialogue.Dialogue_Text` (`|GetArrayItem` (`local.ReturnedLines`)) _aswb_dialogue)
    (else
      (`self.isnotValid`)
      (set `self.LineCurrent` 0)
      (`ActorComponent.Activate` (`Character.CharacterMovement` (`self.MainActor`)) false)
      (if (`self.hasNext`)
        (`self.changeConversation`)))))

(fn `isnotValid`
  (bind _returnvalue (`GameplayStatics.GetPlayerController` 0))
  (bind _foundwidgets (`WidgetBlueprintLibrary.GetAllWidgetsOfClass` "/Game/Blueprints/UI/Dialogue/WB_Dialogue.WB_Dialogue_C" false))
  (for _array_element _foundwidgets
    (`Widget.RemoveFromParent` _array_element))
  (`PlayerController.SetViewTargetWithBlend` _returnvalue (`self.MainActor`) 0.0 "VTBlend_Linear" 0.0 false)
  (`self.EnableInput` _returnvalue)
  (`Widget.SetVisibility` (`self.HUD_Character`) "Visible"))

(fn `UserConstructionScript`)