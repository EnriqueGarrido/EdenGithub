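; BP_Squire is a talking NPC Blueprint for the Squire character.
; On BeginPlay it sets its NPC ID, starting line, conversation ID, speaker name and portrait brush, then calls the parent's BeginPlay.
; Each Interact event increments the current line and calls CreateDialogue to present it.
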(event `self.ReceiveBeginPlay`
  (set `self.NPC_ID` 3)
  (set `self.LineCurrent` 0)
  (set `self.Conversation_ID` 1)
  (set `self.inCharge` "Squire")
  (set `self.Avatar` (make `SlateBrush` (256.0 256.0) (struct) (struct :`SpecifiedColor` (struct :`R` 1.0 :`G` 1.0 :`B` 1.0 :`A` 1.0) :`ColorUseRule` "UseColor_Specified") "/Game/UI/Icons/Characters/Squire.Squire"))
  (`parent.ReceiveBeginPlay`))

(event `/Game/Blueprints/Dialogue/Interact.Interact`
  (`/Engine/EditorBlueprintResources/StandardMacros.IncrementInt` (`self.LineCurrent`)
    (:`  `
      (`self.createDialogue`))))

(fn `UserConstructionScript`
  (`parent.UserConstructionScript`))