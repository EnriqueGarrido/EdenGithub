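; BP_MeleeEnemy is a melee enemy NPC that arms itself when play begins and designates a money bag as its death drop.
; On BeginPlay, after the parent logic, it spawns its Weapon class with itself as instigator and attaches it to the mesh's right-hand socket.
; It then sets MoneyToSpawnOnDeath to BP_MoneyBag; Tick and the construction script only call the parent.
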(event `self.ReceiveBeginPlay`
  (`parent.ReceiveBeginPlay`)
  ;[1 1 1] Attach a weapon
  (bind _returnvalue (`|SpawnActorFromClass` (`self.Weapon`) (`KismetMathLibrary.MakeTransform` (0.0 0.0 -1000.0)) "AlwaysSpawn" "OverrideRootScale" null self))
  (bind _output_get (set `self.CurrentWeapon` _returnvalue))
  (`self.K2_AttachToComponent` _output_get (`self.Mesh`) "hand_rSocket" "SnapToTarget" "SnapToTarget" "KeepWorld" true)
  ;[1 1 1] Set money object
  (set `self.MoneyToSpawnOnDeath` "/Game/Blueprints/Pickups/Money/BP_MoneyBag.BP_MoneyBag_C"))

(event `self.ReceiveTick`
  (params (DeltaSeconds :type "Float (single-precision)"))
  (`parent.ReceiveTick` DeltaSeconds))

(fn `UserConstructionScript`
  (`parent.UserConstructionScript`))