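; Melee weapon actor that detects hits during attack windows and reports them to its wielder through Gameplay Ability System events.
; Begin and end attack events store the event tag and toggle capsule query collision.
; Overlaps with actors of a different class than the instigator send that tag and target, gated by a DoOnce reset shortly after overlap ends.
; Hits can trigger a limited number of brief hit pauses using global time dilation.
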(event `self.ReceiveBeginPlay`
  (`PrimitiveComponent.IgnoreActorWhenMoving` (`self.CapsuleCollision`) null true))

(event `BeginWeaponAttack`
  (params (EventTag :type "GameplayTag Structure") (AttackDelayTime :type "Float (double-precision)") (AttackDelayCount :type Integer))
  (set `self.AttackEventTag` EventTag)
  (set `self.AttackDelayCount` AttackDelayCount)
  (set `self.AttackDelayTime` AttackDelayTime)
  (set `self.bIsAttacking` true)
  (`PrimitiveComponent.SetCollisionEnabled` (`self.CapsuleCollision`) "QueryOnly"))

(event `EndWeaponAttack`
  (set `self.bIsAttacking` false)
  (`PrimitiveComponent.SetCollisionEnabled` (`self.CapsuleCollision`) "NoCollision"))

(event `self.ReceiveActorBeginOverlap`
  (params (OtherActor :type "Actor Object Reference"))
  (bind _returnvalue (`self.GetInstigator`))
  (if (and (!= (`GameplayStatics.GetObjectClass` OtherActor) (`GameplayStatics.GetObjectClass` _returnvalue)) (`self.bIsAttacking`))
    (`/Engine/EditorBlueprintResources/StandardMacros.DoOnce` false :!label _label
      (:`Completed`
        (`AbilitySystemBlueprintLibrary.SendGameplayEventToActor` (`self.GetInstigator`) (`self.AttackEventTag`) (make `GameplayEventData` (struct) _returnvalue OtherActor))
        (`self.HitPause`)))))

(event `self.ReceiveActorEndOverlap`
  (params (OtherActor :type "Actor Object Reference"))
  (`KismetSystemLibrary.Delay` 0.2)
  (goto _label :!via `Reset`))

(event `HitPause`
  (if (and (> (`self.AttackDelayCount`) 0) (`self.bEnableAttackDelay`))
    (`/Engine/EditorBlueprintResources/StandardMacros.DecrementInt` (`self.AttackDelayCount`)
      (:`  `
        (`KismetSystemLibrary.Delay` 0.1)
        (`GameplayStatics.SetGlobalTimeDilation` 0.1)
        (`KismetSystemLibrary.Delay` 0.01)
        (`GameplayStatics.SetGlobalTimeDilation` 1.0)))))

(fn `UserConstructionScript`)